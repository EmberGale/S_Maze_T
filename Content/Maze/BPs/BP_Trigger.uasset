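; BP_Trigger is a placeable trigger volume in the Maze content that starts Niagara effects when the player walks into it.
; When the Box component is overlapped by player character 0, it activates the Niagara component of every entry in the NiagaraToTrigger array, without resetting them.
; The construction script sizes the box from the Length, Width and Height variables.
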(event OnComponentBeginOverlap(Box)
  (params (OverlappedComponent :type Primitive%20Component%20Object%20Reference) (OtherActor :type Actor%20Object%20Reference) (OtherComp :type Primitive%20Component%20Object%20Reference) (OtherBodyIndex :type Integer) (bFromSweep :type Boolean) (SweepResult :type Hit%20Result%20Structure%20%28by%20ref%29))
  (if (== OtherActor (Game|GetPlayerCharacter 0))
    (for _array_element (Variables|Default|GetNiagaraToTrigger)
      (Components|Activation|Activate (Variables|/Script/Niagara.NiagaraActor|GetNiagaraComponent _array_element) false))))

(event EventBeginPlay)

(event Collision|EventActorBeginOverlap
  (params (OtherActor :type Actor%20Object%20Reference)))

(event EventTick
  (params (DeltaSeconds :type Float%20%28single-precision%29)))

(fn ConstructionScript
  (Components|Box|SetBoxExtent (Variables|Default|GetBox) (Math|Vector|MakeVector (Variables|Default|GetLength) (Variables|Default|GetWidth) (Variables|Default|GetHeight)) true))