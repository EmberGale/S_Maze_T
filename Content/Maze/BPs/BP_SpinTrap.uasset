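; BP_SpinTrap is a maze trap with a spinning blade that damages actors touching it.
; Spin plays a timeline that drives the pitch of CustomMesh, and BeginPlay calls it when TriggerOnSpawn is set.
; The Box component applies HitDamage to the other actor on both hit and overlap, printing a debug string each time.
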(event OnComponentHit(Box)
  (params (HitComponent :type Primitive%20Component%20Object%20Reference) (OtherActor :type Actor%20Object%20Reference) (OtherComp :type Primitive%20Component%20Object%20Reference) (NormalImpulse :type Vector :default "0, 0, 0") (Hit :type Hit%20Result%20Structure%20%28by%20ref%29))
  (Development|PrintString "HitBlade")
  (Game|Damage|ApplyDamage OtherActor (Variables|Default|GetHitDamage) 0 0))

(event OnComponentBeginOverlap(Box)
  (params (OverlappedComponent :type Primitive%20Component%20Object%20Reference) (OtherActor :type Actor%20Object%20Reference) (OtherComp :type Primitive%20Component%20Object%20Reference) (OtherBodyIndex :type Integer) (bFromSweep :type Boolean) (SweepResult :type Hit%20Result%20Structure%20%28by%20ref%29))
  (Development|PrintString "OverlapBlade")
  (Game|Damage|ApplyDamage OtherActor (Variables|Default|GetHitDamage) 0 0))

(event Custom|Spin
  (bind _newtrack_0 (Timeline|Timeline Play)
    (:Update
      (Transformation|SetRelativeRotation (Variables|Default|GetCustomMesh) (Math|Rotator|MakeRotator 0.0 _newtrack_0 0.0) false false))))

(event EventBeginPlay
  (if (Variables|Default|GetTriggerOnSpawn)
    (CallFunction|Spin)))

(event Collision|EventActorBeginOverlap
  (params (OtherActor :type Actor%20Object%20Reference)))

(event EventTick
  (params (DeltaSeconds :type Float%20%28single-precision%29)))

(fn ConstructionScript)