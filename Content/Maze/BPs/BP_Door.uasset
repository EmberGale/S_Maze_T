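; BP_Door is an interactable maze door that swings open and shut around its yaw axis.
; Its interaction component's OnInteract event alternates a FlipFlop, compared against Closed to play or reverse a timeline lerping the mesh toward OpenAngle.
; The construction script pre-rotates doors that spawn open and calls an event meant to set the timeline time.
; Overlapping the door mesh shows two text renders to the player character.
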(event OnInteract(BP_InteractionComponent)
  (params (bActivation :type Boolean))
  (bind _isa (Utilities|FlowControl|FlipFlop)
    (:A
      _)
    (:B
      _))
  (if (== _isa (Variables|Default|GetClosed))
    (bind _newtrack_0 (Timeline|Timeline Play)
      (:Update
        (Transformation|SetRelativeRotation (Variables|Default|GetSM_door_03) (Math|Rotator|MakeRotator 0.0 0.0 (Math|Float|Lerp 0.0 (Variables|Default|GetOpenAngle) _newtrack_0)) false false)))
    (else
      (Timeline|Timeline Reverse))))

(event OnComponentBeginOverlap(SM_door_03)
  (params (OverlappedComponent :type Primitive%20Component%20Object%20Reference) (OtherActor :type Actor%20Object%20Reference) (OtherComp :type Primitive%20Component%20Object%20Reference) (OtherBodyIndex :type Integer) (bFromSweep :type Boolean) (SweepResult :type Hit%20Result%20Structure%20%28by%20ref%29))
  (if (== OtherActor (Game|GetPlayerCharacter 0))
    (Rendering|SetVisibility (Variables|Default|GetTextRender1) true false)
    (Rendering|SetVisibility (Variables|Default|GetTextRender) true false)))

(event OnComponentEndOverlap(SM_door_03)
  (params (OverlappedComponent :type Primitive%20Component%20Object%20Reference) (OtherActor :type Actor%20Object%20Reference) (OtherComp :type Primitive%20Component%20Object%20Reference) (OtherBodyIndex :type Integer))
  (if (== (Game|GetPlayerCharacter 0) OtherActor)
    (Rendering|SetVisibility (Variables|Default|GetTextRender1) false false)
    (Rendering|SetVisibility (Variables|Default|GetTextRender) false false)))

(event Custom|SetTimeTimeline
  (params (Time :type Float%20%28double-precision%29))
  (bind _newtrack_0 (Timeline|Timeline SetNewTime)
    (:Update
      (Transformation|SetRelativeRotation (Variables|Default|GetSM_door_03) (Math|Rotator|MakeRotator 0.0 0.0 (Math|Float|Lerp 0.0 (Variables|Default|GetOpenAngle) _newtrack_0)) false false))))

(event EventBeginPlay)

(fn ConstructionScript
  ;[0.0137 0.01161 0.009134] If Door Opened on Spawn
  (if (not (Variables|Default|GetClosed))
    (Transformation|SetRelativeRotation (Variables|Default|GetSM_door_03) (Math|Rotator|MakeRotator 0.0 0.0 (Variables|Default|GetOpenAngle)) false true)
    (CallFunction|SetTimeTimeline 1.0)))