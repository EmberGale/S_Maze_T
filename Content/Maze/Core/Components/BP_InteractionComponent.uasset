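; BP_InteractionComponent is a component that holds interactable and activated state for whatever actor carries it.
; Enable and disable events set the Interactable flag and broadcast OnToggleInteractability.
; Interact works only while Interactable is true, flipping Activated like a toggle switch and broadcasting OnInteract with the new state.
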(event Custom|EnableInteractability
  ;[0.2656 0.09522 0.1872] Enable / Disable Interactability
  (Variables|Default|SetbInteractable true)
  (Default|CallOnToggleInteractability))

(event Custom|DisableInteractability
  ;[0.2656 0.09522 0.1872] Enable / Disable Interactability
  (Variables|Default|SetbInteractable false)
  (Default|CallOnToggleInteractability))

(event Custom|Interact
  (if (Variables|Default|GetbInteractable)
    (bind _output_get (Variables|Default|SetbActivated (not (Variables|Default|GetbActivated))))
    (Default|CallOnInteract _output_get)))