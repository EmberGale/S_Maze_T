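; Health component for the Maze game that tracks its owner's health and keeps the player HUD in sync.
; On BeginPlay it binds to the owner's any-damage event and caches player 0's HUD_Maze.
; ChangeHealth adds a signed delta, clamped to zero and max, then refreshes the HUD, while SetHealth skips both.
; Damage passes in un-negated, and OnDeath fires when health reaches zero.
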(event Custom|OnTakeAnyDamage_Event
  (params (DamagedActor :type Actor%20Object%20Reference) (Damage :type Float%20%28single-precision%29) (DamageType :type Damage%20Type%20Object%20Reference) (InstigatedBy :type Controller%20Object%20Reference) (DamageCauser :type Actor%20Object%20Reference))
  (CallFunction|ChangeHealth Damage)
  (if (<= (CallFunction|GetHealth) 0.0)
    (Default|CallOnDeath)))

(event EventBeginPlay
  (EventDispatchers|AssignOnTakeAnyDamage (Components|GetOwner) (delegate Custom|OnTakeAnyDamage_Event))
  (bind _ashud_maze (Utilities|Casting|CastToHUD_Maze (HUD|GetHUD (Game|GetPlayerController 0))))
  (bind _output_get (Variables|Default|SetAs%20HUD%20Maze _ashud_maze))
  (Default|UpdateHealth _output_get))

(fn GetHealth
  (return (Variables|Default|GetHealth)))

(fn SetHealth
  (params (Health :type Float%20%28double-precision%29))
  (Variables|Default|SetHealth Health))

(fn ChangeHealth
  (params (Change :type Float%20%28double-precision%29))
  (Variables|Default|SetHealth (Math|Float|Clamp(Float) (+ Change (Variables|Default|GetHealth)) 0.0 (Variables|Default|GetMaxHealth)))
  (Default|UpdateHealth (Variables|Default|GetAs%20HUD%20Maze)))

(fn GetMaxHealth
  (return (Variables|Default|GetMaxHealth)))